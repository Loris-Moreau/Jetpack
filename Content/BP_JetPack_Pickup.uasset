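; BP_JetPack_Pickup is a jetpack pickup actor that bobs and spins until the third-person character overlaps its box.
; Tick yaws it and moves it along local Z, with a Delay feeding a FlipFlop that periodically reverses the direction.
; Overlap by BP_ThirdPersonCharacter sets HasBeenPickedUp, stopping the motion, then destroys the actor after a delay.
; The graph itself does not grant the jetpack to the character.
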(event `self.ReceiveBeginPlay`)

(event `self.ReceiveTick`
  (params (DeltaSeconds :type "Float (single-precision)"))
  (if (not (`self.Has Been Picked Up`))
    (`|ExecutionSequence`
      (:`then_0`
        (`KismetSystemLibrary.Delay` (`self.Pickup Swing Delay`))
        (bind _isa (`/Engine/EditorBlueprintResources/StandardMacros.FlipFlop`)
          (:`A`
            _)
          (:`B`
            _))
        (set `self.Dir` _isa))
      (:`then_1`
        (if (`self.Dir`)
          (`self.K2_AddActorLocalOffset` (`KismetMathLibrary.MakeVector` 0.0 0.0 (`self.Pickup Offset`)))
          (else
            (`self.K2_AddActorLocalOffset` (`KismetMathLibrary.MakeVector` 0.0 0.0 (* (`self.Pickup Offset`) -1.0))))))
      (:`then_2`
        (`self.K2_AddActorLocalRotation` (`KismetMathLibrary.MakeRotator` 0.0 0.0 (`self.Pickup Rotation`)))))))

(event `self.Box.OnComponentBeginOverlap`
  (params (OverlappedComponent :type "PrimitiveComponent Object Reference") (OtherActor :type "Actor Object Reference") (OtherComp :type "PrimitiveComponent Object Reference") (OtherBodyIndex :type Integer) (bFromSweep :type Boolean) (SweepResult :type "HitResult Structure (by ref)"))
  (bind _asbp_third_person_character (cast `/Game/ThirdPerson/Blueprints/BP_ThirdPersonCharacter` OtherActor))
  (if (== _asbp_third_person_character OtherActor)
    (set `self.Has Been Picked Up` true)
    (`KismetSystemLibrary.Delay` (`self.Destroy Delay`))
    (`self.K2_DestroyActor`)))

(fn `UserConstructionScript`)