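; BP_Enemy_Spot_3 is an enemy whose eye mesh continuously turns to face the player's spaceship.
; On BeginPlay it finds the BP_Spaceship actor and stores its Billboard component as the look-at target.
; Each Tick, while that target is valid, it snaps SMEye's world rotation toward the target's location, without interpolation.
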(event `self.ReceiveBeginPlay`
  (`parent.ReceiveBeginPlay`)
  (bind _returnvalue (`GameplayStatics.GetActorOfClass` "/Game/Spaceship/BP_Spaceship.BP_Spaceship_C"))
  (set `self.Enemy Look At` (`/Game/Spaceship/BP_Spaceship.Billboard` _returnvalue)))

(event `self.ReceiveTick`
  (params (DeltaSeconds :type "Float (single-precision)"))
  (bind _sm_eye (`self.SM_Eye`))
  (bind _enemy_look_at (`self.Enemy Look At`))
  (`parent.ReceiveTick` DeltaSeconds)
  (`/Engine/EditorBlueprintResources/StandardMacros.IsValid` _enemy_look_at
    (:`Is Valid`
      (`SceneComponent.K2_SetWorldRotation` _sm_eye (`KismetMathLibrary.FindLookAtRotation` (`SceneComponent.K2_GetComponentLocation` _sm_eye) (`SceneComponent.K2_GetComponentLocation` _enemy_look_at)) false false))))

(fn `UserConstructionScript`
  (`parent.UserConstructionScript`))