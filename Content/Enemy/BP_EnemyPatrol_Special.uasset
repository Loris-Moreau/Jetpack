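; BP_EnemyPatrol_Special is an enemy variant that rewards the player for a head stomp or dash hit and notifies a ScreenTrigger.
; KillHeadBox overlaps add stomp score, while KillBox overlaps add dash score only if the player is dashing.
; Both paths then bounce the player, play a sound, restore dashing and, after a short delay, pass the enemy to ScreenTrigger.UpdateScreen.
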(event `self.Kill Head Box.OnComponentBeginOverlap`
  (params (OverlappedComponent :type "PrimitiveComponent Object Reference") (OtherActor :type "Actor Object Reference") (OtherComp :type "PrimitiveComponent Object Reference") (OtherBodyIndex :type Integer) (bFromSweep :type Boolean) (SweepResult :type "HitResult Structure (by ref)"))
  (bind _asbp_third_person_character (cast `/Game/ThirdPerson/Blueprints/BP_ThirdPersonCharacter` (`GameplayStatics.GetPlayerCharacter` 0) :!pure true))
  (if (`self.ActorHasTag` OtherActor "Player")
    (set `/Game/ThirdPerson/Blueprints/BP_ThirdPersonCharacter.Score` (+ (`/Game/ThirdPerson/Blueprints/BP_ThirdPersonCharacter.Score` _asbp_third_person_character) (`self.Score Kill Enemy`)) _asbp_third_person_character)
    (`Character.LaunchCharacter` _asbp_third_person_character (`KismetMathLibrary.MakeVector` 0.0 0.0 (`self.Bounce Force`)) false false :!label _label)
    ;[0 1 0.03793] Sound
    (`GameplayStatics.PlaySoundAtLocation` null (0.0 0.0 0.0) (struct) 1.0 1.0 0.0 null null null null)
    (set `/Game/ThirdPerson/Blueprints/BP_ThirdPersonCharacter.Can Dash` true _asbp_third_person_character)
    (`KismetSystemLibrary.Delay` 0.2)
    (`/Game/MapElements/BP_ScreenTrigger.UpdateScreen` (`self.ScreenTrigger`) self)))

(event `self.KillBox.OnComponentBeginOverlap`
  (params (OverlappedComponent :type "PrimitiveComponent Object Reference") (OtherActor :type "Actor Object Reference") (OtherComp :type "PrimitiveComponent Object Reference") (OtherBodyIndex :type Integer) (bFromSweep :type Boolean) (SweepResult :type "HitResult Structure (by ref)"))
  (bind _asbp_third_person_character (cast `/Game/ThirdPerson/Blueprints/BP_ThirdPersonCharacter` (`GameplayStatics.GetPlayerCharacter` 0) :!pure true))
  ;[1 1 1] Kill With Dash
  (if (and (`self.ActorHasTag` OtherActor "Player") (`/Game/ThirdPerson/Blueprints/BP_ThirdPersonCharacter.IsDashing` (cast `/Game/ThirdPerson/Blueprints/BP_ThirdPersonCharacter` (`GameplayStatics.GetPlayerCharacter` 0) :!pure true)))
    (set `/Game/ThirdPerson/Blueprints/BP_ThirdPersonCharacter.Score` (+ (`/Game/ThirdPerson/Blueprints/BP_ThirdPersonCharacter.Score` _asbp_third_person_character) (`self.Score Kill Dash`)) _asbp_third_person_character)
    (goto _label)))

(fn `UserConstructionScript`
  (`parent.UserConstructionScript`))