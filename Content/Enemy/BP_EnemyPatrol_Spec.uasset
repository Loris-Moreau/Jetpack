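; Patrol enemy that moves along the level's BP_Spline and can be killed by the player for score.
; A timeline, scaled by TimeToComplete, drives its position along the spline once MoveObject is called.
; A head stomp bounces the player; body contact kills the enemy if dashing, otherwise costs health.
; Kills remove both hitboxes, swap the cube for score text, restore dash and update ScreenTrigger.
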(event `Destroy Box Score`
  (`ActorComponent.K2_DestroyComponent` (`self.Kill Head Box`))
  (`ActorComponent.K2_DestroyComponent` (`self.KillBox`)))

(event `Show Score Dash Kill`
  (bind _scoretxt (`self.ScoreTXT`))
  (`TextRenderComponent.K2_SetText` _scoretxt (`|FormatText` "+ {score}" (`self.Score Kill Dash`)))
  (`SceneComponent.SetVisibility` _scoretxt true false)
  (`SceneComponent.SetVisibility` (`self.Cube`) false false)
  (`TimelineComponent.Stop` (`self.MoveObjectT`)))

(event `Show Score Kill`
  (bind _scoretxt (`self.ScoreTXT`))
  (`TextRenderComponent.K2_SetText` _scoretxt (`|FormatText` "+ {score}" (`self.Score Kill Enemy`)))
  (`SceneComponent.SetVisibility` _scoretxt true false)
  (`SceneComponent.SetVisibility` (`self.Cube`) false false)
  (`TimelineComponent.Stop` (`self.MoveObjectT`)))

(event `self.ReceiveBeginPlay`
  ;[1 1 1] Define Spline REF
  (bind _returnvalue (`GameplayStatics.GetActorOfClass` "/Game/Enemy/BP_Spline.BP_Spline_C"))
  (set `self.SplineREF` _returnvalue)
  (`SceneComponent.SetVisibility` (`self.ScoreTXT`) false false))

(event `Move Object`
  ;[1 1 1] Move Enemy on Spline
  (`TimelineComponent.SetPlayRate` (`self.MoveObjectT`) (/ 1.0 (`self.Time To Complete`)))
  (bind (_direction _movetrack) (`Timeline|MoveObjectT`)
    (:`Update`
      (`self.K2_SetActorTransform` (`KismetMathLibrary.MakeTransform` (`SplineComponent.GetLocationAtDistanceAlongSpline` (`/Game/Enemy/BP_Spline.Spline` (`self.SplineREF`)) (`KismetMathLibrary.Lerp` 0.0 (`SplineComponent.GetSplineLength` (`/Game/Enemy/BP_Spline.Spline` (`self.SplineREF`))) _movetrack) "World"))))))

(event `self.Kill Head Box.OnComponentBeginOverlap`
  (params (OverlappedComponent :type "PrimitiveComponent Object Reference") (OtherActor :type "Actor Object Reference") (OtherComp :type "PrimitiveComponent Object Reference") (OtherBodyIndex :type Integer) (bFromSweep :type Boolean) (SweepResult :type "HitResult Structure (by ref)"))
  (bind _asbp_third_person_character (cast `/Game/ThirdPerson/Blueprints/BP_ThirdPersonCharacter` (`GameplayStatics.GetPlayerCharacter` 0) :!pure true))
  (bind (_velocity_x _velocity_y _velocity_z) (`KismetMathLibrary.BreakVector` (`MovementComponent.Velocity` (`Character.CharacterMovement` (cast `/Game/ThirdPerson/Blueprints/BP_ThirdPersonCharacter` (`GameplayStatics.GetPlayerCharacter` 0) :!pure true)))))
  (if (`self.ActorHasTag` OtherActor "Player")
    ;[1 1 1] Add Scoring Sys
    (set `/Game/ThirdPerson/Blueprints/BP_ThirdPersonCharacter.Score` (+ (`/Game/ThirdPerson/Blueprints/BP_ThirdPersonCharacter.Score` _asbp_third_person_character) (`self.Score Kill Enemy`)) _asbp_third_person_character)
    (`self.Destroy Box Score`)
    (`self.Show Score Kill`)
    (`Character.LaunchCharacter` _asbp_third_person_character (`KismetMathLibrary.MakeVector` 0.0 0.0 (+ (`self.Bounce Force`) (`KismetMathLibrary.Abs` _velocity_z))) false false)
    ;[0 1 0.03793] Sound
    (`GameplayStatics.PlaySoundAtLocation` null (0.0 0.0 0.0) (struct) 1.0 1.0 0.0 null null null null :!label _label)
    (`KismetSystemLibrary.Delay` 0.2)
    (set `/Game/ThirdPerson/Blueprints/BP_ThirdPersonCharacter.Can Dash` true _asbp_third_person_character)
    (`/Game/MapElements/BP_ScreenTrigger.UpdateScreen` (`self.ScreenTrigger`) self)))

(event `self.KillBox.OnComponentBeginOverlap`
  (params (OverlappedComponent :type "PrimitiveComponent Object Reference") (OtherActor :type "Actor Object Reference") (OtherComp :type "PrimitiveComponent Object Reference") (OtherBodyIndex :type Integer) (bFromSweep :type Boolean) (SweepResult :type "HitResult Structure (by ref)"))
  (bind _asbp_third_person_character (cast `/Game/ThirdPerson/Blueprints/BP_ThirdPersonCharacter` (`GameplayStatics.GetPlayerCharacter` 0) :!pure true))
  (bind _asbp_third_person_character_2 (cast `/Game/ThirdPerson/Blueprints/BP_ThirdPersonCharacter` (`GameplayStatics.GetPlayerCharacter` 0) :!pure true))
  ;[1 1 1] Kill With Dash
  (if (`self.ActorHasTag` OtherActor "Player")
    (if (`/Game/ThirdPerson/Blueprints/BP_ThirdPersonCharacter.IsDashing` _asbp_third_person_character_2)
      (set `/Game/ThirdPerson/Blueprints/BP_ThirdPersonCharacter.Score` (+ (`/Game/ThirdPerson/Blueprints/BP_ThirdPersonCharacter.Score` _asbp_third_person_character) (`self.Score Kill Dash`)) _asbp_third_person_character)
      (`self.Destroy Box Score`)
      (`self.Show Score Dash Kill`)
      (goto _label)
      (else
        (`/Game/ThirdPerson/Blueprints/BP_ThirdPersonCharacter.Decrement Health` _asbp_third_person_character_2)))))

(fn `UserConstructionScript`)