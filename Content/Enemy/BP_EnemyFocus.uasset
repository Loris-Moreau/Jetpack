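; BP_EnemyFocus is an enemy pawn that chases the player after a startup delay.
; BeginPlay waits for TimeBeforeFocus, then sets the TimeFinished flag.
; Once the flag is set, Tick reissues AIMoveTo every frame toward the current location of the player's BP_ThirdPersonCharacter, using a small acceptance radius.
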(event `self.ReceiveBeginPlay`
  (`KismetSystemLibrary.Delay` (`self.Time Before Focus`))
  (set `self.TimeFinished` true))

(event `self.ReceiveTick`
  (params (DeltaSeconds :type "Float (single-precision)"))
  (bind _returnvalue_location (`KismetMathLibrary.BreakTransform` (`self.GetTransform` (cast `/Game/ThirdPerson/Blueprints/BP_ThirdPersonCharacter` (`GameplayStatics.GetPlayerCharacter` 0) :!pure true))))
  (if (`self.TimeFinished`)
    (`|AIMoveTo` self _returnvalue_location null 2.0)))

(fn `UserConstructionScript`)