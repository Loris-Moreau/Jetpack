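; Enemy spawner that, between StartSpawn and StopSpawn, places BP_EnemySpot enemies at random points along a spline.
; After an initial delay, three self-recalling loops each read their DataTable row, roll its probability, spawn and enable that enemy, then wait SpawnDelay.
; A looping timer periodically shortens SpawnDelay toward a floor to raise difficulty.
; StopSpawn calls DieFeedbacks on all BP_EnemySpot actors and clears CanSpawn to end the loops.
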(event `self.ReceiveBeginPlay`)

(event `IncreseDifficulty`
  (bind _spawn_delay_ (`self.Spawn Delay `))
  (if (not (<= _spawn_delay_ 0.35))
    (bind _output_get (set `self.Spawn Delay ` (- _spawn_delay_ 0.05)))
    (`KismetSystemLibrary.PrintString` (`KismetStringLibrary.Conv_DoubleToString` _output_get))))

(event `StartSpawn`
  (set `self.CanSpawn?` true)
  (`KismetSystemLibrary.K2_SetTimerDelegate` (delegate `IncreseDifficulty`) 10.0 true)
  (`KismetSystemLibrary.Delay` (`self.Delay for first spawn`))
  (`|ExecutionSequence`
    (:`then_0`
      (`self.Spawn Enemy 1`))
    (:`then_1`
      (`self.Spawn Enemy 2`))
    (:`then_2`
      (`self.SpawnEnemy3`))))

(event `Spawn Enemy 1`
  (bind _datatable_ref (`self.DataTable Ref`))
  (bind _spline (`self.Spline`))
  (if (`self.CanSpawn?`)
    (bind _outrownames (`DataTableFunctionLibrary.GetDataTableRowNames` _datatable_ref))
    (bind _returnvalue (`|GetDataTableRow` _datatable_ref (`|GetArrayItem` _outrownames))
      (:`then`
        (bind (_enemy `_probabilité`) (break `/Game/Enemy/S_Enemy` _returnvalue))
        (bind _output_get (set `self.Spawn Proba Enemy 1` `_probabilité`))
        (if (<= (`KismetMathLibrary.RandomFloatInRange` 0.0 1.0) _output_get)
          ;[1 1 1] Spawn
          (bind _returnvalue_2 (`|SpawnActorFromClass` _enemy (`KismetMathLibrary.MakeTransform` (`SplineComponent.GetLocationAtDistanceAlongSpline` _spline (`KismetMathLibrary.RandomFloatInRange` 0.0 (`SplineComponent.GetSplineLength` _spline)) "World")) "AdjustIfPossibleButDontSpawnIfColliding" "MultiplyWithRoot" null null))
          (bind _asbp_enemy_spot (cast `/Game/Enemy/Olds/BP_EnemySpot` _returnvalue_2))
          (set `/Game/Enemy/Olds/BP_EnemySpot.Enabled` true _asbp_enemy_spot))
        (`KismetSystemLibrary.Delay` (`self.Spawn Delay `))
        (`self.Spawn Enemy 1`)))))

(event `Spawn Enemy 2`
  (bind _datatable_ref (`self.DataTable Ref`))
  (bind _spline (`self.Spline`))
  (if (`self.CanSpawn?`)
    (bind _outrownames (`DataTableFunctionLibrary.GetDataTableRowNames` _datatable_ref))
    (bind _returnvalue (`|GetDataTableRow` _datatable_ref (`|GetArrayItem` _outrownames 1))
      (:`then`
        (bind (_enemy `_probabilité`) (break `/Game/Enemy/S_Enemy` _returnvalue))
        (bind _output_get (set `self.Spawn Proba Enemy 2` `_probabilité`))
        (if (<= (`KismetMathLibrary.RandomFloatInRange` 0.0 1.0) _output_get)
          ;[1 1 1] Spawn
          (bind _returnvalue_2 (`|SpawnActorFromClass` _enemy (`KismetMathLibrary.MakeTransform` (`SplineComponent.GetLocationAtDistanceAlongSpline` _spline (`KismetMathLibrary.RandomFloatInRange` 0.0 (`SplineComponent.GetSplineLength` _spline)) "World")) "AdjustIfPossibleButDontSpawnIfColliding" "MultiplyWithRoot" null null))
          (bind _asbp_enemy_spot (cast `/Game/Enemy/Olds/BP_EnemySpot` _returnvalue_2))
          (set `/Game/Enemy/Olds/BP_EnemySpot.Enabled` true _asbp_enemy_spot))
        (`KismetSystemLibrary.Delay` (`self.Spawn Delay `))
        (`self.Spawn Enemy 2`)))))

(event `SpawnEnemy3`
  (bind _datatable_ref (`self.DataTable Ref`))
  (bind _spline (`self.Spline`))
  (if (`self.CanSpawn?`)
    (bind _outrownames (`DataTableFunctionLibrary.GetDataTableRowNames` _datatable_ref))
    (bind _returnvalue (`|GetDataTableRow` _datatable_ref (`|GetArrayItem` _outrownames 2))
      (:`then`
        (bind (_enemy `_probabilité`) (break `/Game/Enemy/S_Enemy` _returnvalue))
        (bind _output_get (set `self.Spawn Proba Enemy 2` `_probabilité`))
        (if (<= (`KismetMathLibrary.RandomFloatInRange` 0.0 1.0) _output_get)
          (bind _returnvalue_2 (`|SpawnActorFromClass` _enemy (`KismetMathLibrary.MakeTransform` (`SplineComponent.GetLocationAtDistanceAlongSpline` _spline (`KismetMathLibrary.RandomFloatInRange` 0.0 (`SplineComponent.GetSplineLength` _spline)) "World")) "AdjustIfPossibleButDontSpawnIfColliding" "MultiplyWithRoot" null null))
          (bind _asbp_enemy_spot (cast `/Game/Enemy/Olds/BP_EnemySpot` _returnvalue_2))
          (set `/Game/Enemy/Olds/BP_EnemySpot.Enabled` true _asbp_enemy_spot))
        (`KismetSystemLibrary.Delay` (`self.Spawn Delay `))
        (`self.SpawnEnemy3`)))))

(event `StopSpawn`
  (bind _outactors (`GameplayStatics.GetAllActorsOfClass` "/Game/Enemy/Olds/BP_EnemySpot.BP_EnemySpot_C"))
  (for _array_element _outactors
    (`/Game/Enemy/Olds/BP_EnemySpot.DieFeedbacks` _array_element))
  (set `self.CanSpawn?` false))

(fn `UserConstructionScript`)