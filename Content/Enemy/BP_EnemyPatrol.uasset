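; Patrolling enemy that moves along a spline and can be stomped by the player through its KillHeadBox.
; BeginPlay grabs the first BP_Spline in the level, and MoveObject plays a timeline scaled by TimeToComplete to set location and rotation along it.
; Any head-box overlap adds score to the player character, launches it upward, plays a sound, then after a short delay passes itself to ScreenTrigger.UpdateScreen.
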(event `self.ReceiveBeginPlay`
  ;[1 1 1] Define Spline REF
  (bind _returnvalue (`GameplayStatics.GetActorOfClass` "/Game/Enemy/BP_Spline.BP_Spline_C"))
  (set `self.SplineREF` _returnvalue))

(event `Move Object`
  (bind _spline (`/Game/Enemy/BP_Spline.Spline` (`self.SplineREF`)))
  ;[1 1 1] Move Enemy on Spline
  (`TimelineComponent.SetPlayRate` (`self.MoveObjectT`) (/ 1.0 (`self.Time To Complete`)))
  (bind (_direction _movetrack) (`Timeline|MoveObjectT`)
    (:`Update`
      (bind _returnvalue (`KismetMathLibrary.Lerp` 0.0 (`SplineComponent.GetSplineLength` (`/Game/Enemy/BP_Spline.Spline` (`self.SplineREF`))) _movetrack))
      (`self.K2_SetActorTransform` (`KismetMathLibrary.MakeTransform` (`SplineComponent.GetLocationAtDistanceAlongSpline` _spline _returnvalue "World") (`SplineComponent.GetRotationAtDistanceAlongSpline` _spline _returnvalue "Local"))))))

(event `self.Kill Head Box.OnComponentBeginOverlap`
  (params (OverlappedComponent :type "PrimitiveComponent Object Reference") (OtherActor :type "Actor Object Reference") (OtherComp :type "PrimitiveComponent Object Reference") (OtherBodyIndex :type Integer) (bFromSweep :type Boolean) (SweepResult :type "HitResult Structure (by ref)"))
  (bind _asbp_third_person_character (cast `/Game/ThirdPerson/Blueprints/BP_ThirdPersonCharacter` (`GameplayStatics.GetPlayerCharacter` 0) :!pure true))
  ;[1 1 1] Add Scoring Sys
  (set `/Game/ThirdPerson/Blueprints/BP_ThirdPersonCharacter.Score` (+ (`/Game/ThirdPerson/Blueprints/BP_ThirdPersonCharacter.Score` _asbp_third_person_character) (`self.Score Kill Enemy`)) _asbp_third_person_character)
  (`Character.LaunchCharacter` _asbp_third_person_character (`KismetMathLibrary.MakeVector` 0.0 0.0 (`self.Bounce Force`)) false false)
  ;[0 1 0.03793] Sound
  (`GameplayStatics.PlaySoundAtLocation` null (0.0 0.0 0.0) (struct) 1.0 1.0 0.0 null null null null)
  (`KismetSystemLibrary.Delay` 0.2)
  (`/Game/MapElements/BP_ScreenTrigger.UpdateScreen` (`self.ScreenTrigger`) self))

(fn `UserConstructionScript`)