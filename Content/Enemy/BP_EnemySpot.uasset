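; Enemy character that, while enabled, chases the player and awards points when stomped or dashed into.
; Tick re-issues MoveComponentTo toward the player, with duration set by distance over EnemySpeed.
; HeadKillBox overlaps launch the player upward, while KillBox overlaps count only during a dash.
; Both kills add score, remove the kill boxes, swap the cube for score text, play a sound and notify ScreenTrigger after a short delay.
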(event `Destroy Box Score`
  (`ActorComponent.K2_DestroyComponent` (`self.KillBox`))
  (`ActorComponent.K2_DestroyComponent` (`self.Head Kill Box`)))

(event `Show Score Dash Kill`
  (bind _scoretxt (`self.ScoreTXT`))
  (`TextRenderComponent.K2_SetText` _scoretxt (`|FormatText` "+ {score}" (`self.Score Kill Dash`)))
  (`SceneComponent.SetVisibility` _scoretxt true false)
  (`SceneComponent.SetVisibility` (`self.Cube`) false false))

(event `Show Score Kill`
  (bind _scoretxt (`self.ScoreTXT`))
  (`TextRenderComponent.K2_SetText` _scoretxt (`|FormatText` "+ {score}" (`self.Score Kill Enemy`)))
  (`SceneComponent.SetVisibility` _scoretxt true false)
  (`SceneComponent.SetVisibility` (`self.Cube`) false false))

(event `self.ReceiveBeginPlay`
  (`SceneComponent.SetVisibility` (`self.ScoreTXT`) false false))

(event `self.ReceiveTick`
  (params (DeltaSeconds :type "Float (single-precision)"))
  (bind _returnvalue (`self.K2_GetActorLocation` (`GameplayStatics.GetPlayerCharacter` 0)))
  ;[1 1 1] Move
  (if (`self.Enabled`)
    (`KismetSystemLibrary.MoveComponentTo` (`self.CapsuleComponent`) _returnvalue (struct) false false (/ (`KismetMathLibrary.VSize` (- (`self.K2_GetActorLocation`) _returnvalue)) (`self.Enemy Speed`)))))

(event `self.Head Kill Box.OnComponentBeginOverlap`
  (params (OverlappedComponent :type "PrimitiveComponent Object Reference") (OtherActor :type "Actor Object Reference") (OtherComp :type "PrimitiveComponent Object Reference") (OtherBodyIndex :type Integer) (bFromSweep :type Boolean) (SweepResult :type "HitResult Structure (by ref)"))
  (bind _asbp_third_person_character (cast `/Game/ThirdPerson/Blueprints/BP_ThirdPersonCharacter` (`GameplayStatics.GetPlayerCharacter` 0) :!pure true))
  (bind (_velocity_x _velocity_y _velocity_z) (`KismetMathLibrary.BreakVector` (`MovementComponent.Velocity` (`Character.CharacterMovement` (cast `/Game/ThirdPerson/Blueprints/BP_ThirdPersonCharacter` (`GameplayStatics.GetPlayerCharacter` 0) :!pure true)))))
  (if (`self.ActorHasTag` OtherActor "Player")
    (set `/Game/ThirdPerson/Blueprints/BP_ThirdPersonCharacter.Score` (+ (`/Game/ThirdPerson/Blueprints/BP_ThirdPersonCharacter.Score` _asbp_third_person_character) (`self.Score Kill Enemy`)) _asbp_third_person_character)
    (`self.Destroy Box Score`)
    (`self.Show Score Kill`)
    (`self.LaunchCharacter` _asbp_third_person_character (`KismetMathLibrary.MakeVector` 0.0 0.0 (+ (`self.Bounce Force`) (`KismetMathLibrary.Abs` _velocity_z))) false false)
    ;[0 1 0.03793] Sound
    (`GameplayStatics.PlaySoundAtLocation` null (0.0 0.0 0.0) (struct) 1.0 1.0 0.0 null null null null :!label _label)
    (`KismetSystemLibrary.Delay` 0.2)
    (`/Game/MapElements/BP_ScreenTrigger.UpdateScreen` (`self.ScreenTrigger`) self)))

(event `self.KillBox.OnComponentBeginOverlap`
  (params (OverlappedComponent :type "PrimitiveComponent Object Reference") (OtherActor :type "Actor Object Reference") (OtherComp :type "PrimitiveComponent Object Reference") (OtherBodyIndex :type Integer) (bFromSweep :type Boolean) (SweepResult :type "HitResult Structure (by ref)"))
  (bind _asbp_third_person_character (cast `/Game/ThirdPerson/Blueprints/BP_ThirdPersonCharacter` (`GameplayStatics.GetPlayerCharacter` 0) :!pure true))
  ;[1 1 1] Kill With Dash
  (if (and (`self.ActorHasTag` OtherActor "Player") (`/Game/ThirdPerson/Blueprints/BP_ThirdPersonCharacter.IsDashing` (cast `/Game/ThirdPerson/Blueprints/BP_ThirdPersonCharacter` (`GameplayStatics.GetPlayerCharacter` 0) :!pure true)))
    (set `/Game/ThirdPerson/Blueprints/BP_ThirdPersonCharacter.Score` (+ (`/Game/ThirdPerson/Blueprints/BP_ThirdPersonCharacter.Score` _asbp_third_person_character) (`self.Score Kill Dash`)) _asbp_third_person_character)
    (`self.Destroy Box Score`)
    (`self.Show Score Dash Kill`)
    (goto _label)))

(fn `UserConstructionScript`)