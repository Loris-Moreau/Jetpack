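; Enemy for the jetpack game that, once enabled, moves toward the player pawn at a distance-scaled duration.
; Head stomps bounce the character and, like projectiles, kill it, award score and update its ScreenTrigger.
; Body contact costs player health, repulsing the character or damaging a non-invincible spaceship and killing the enemy.
; Death plays sound, timeline-driven scale-up and material dissolve, then spawns Niagara FX and a score widget before destroying the actor.
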(event `Player Repulse Hit Enemy`
  (bind _returnvalue (`GameplayStatics.GetPlayerPawn` 0))
  (bind (_returnvalue_x _returnvalue_y) (`KismetMathLibrary.BreakVector` (`SceneComponent.GetForwardVector` (`Actor.RootComponent` _returnvalue))))
  ;[1 1 1] Repusle Player
  (bind _player_ref (`self.Player Ref`)
    (:`then`
      (`self.LaunchCharacter` _player_ref (`KismetMathLibrary.MakeVector` 0.0 (* 50.0 _returnvalue_y)) true true))
    (:`else`
      (bind _asbp_spaceship (cast `/Game/Spaceship/BP_Spaceship` _returnvalue))
      (`/Game/Spaceship/BP_Spaceship.TakeDamage` _asbp_spaceship)
      (`self.DieFeedbacks`))))

(event `Stop Movement`
  ;[1 1 1] Stop Move
  (set `self.StopMovement` true)
  (if (`self.Enabled`)
    (`KismetSystemLibrary.MoveComponentTo` (`self.CapsuleComponent`) (`self.K2_GetActorLocation`))))

(event `Destroy Box Score`
  ;[1 1 1] Destroy the Collision boxes when hit
  (`ActorComponent.K2_DestroyComponent` (`self.KillBox`))
  (`ActorComponent.K2_DestroyComponent` (`self.Head Kill Box`)))

(event `Show Score Dash Kill`
  (bind _scoretxt (`self.ScoreTXT`))
  ;[1 1 1] Score Updating
  (`TextRenderComponent.K2_SetText` _scoretxt (`|FormatText` "+ {score}" (`self.Score Kill Dash`)))
  (`SceneComponent.SetVisibility` _scoretxt true false)
  (`SceneComponent.SetVisibility` (`self.Cube`) false false)
  (`self.Stop Movement`))

(event `Show Score Kill`
  (bind _scoretxt (`self.ScoreTXT`))
  ;[1 1 1] Score Updating
  (`TextRenderComponent.K2_SetText` _scoretxt (`|FormatText` "+ {score}" (`self.Score Kill Enemy`)))
  (`SceneComponent.SetVisibility` _scoretxt true false)
  (`SceneComponent.SetVisibility` (`self.Cube`) false false)
  (`self.Stop Movement`))

(event `self.ReceiveBeginPlay`
  ;[1 1 1] Begin play ; Basic References
  (`SceneComponent.SetVisibility` (`self.ScoreTXT`) false false)
  (bind _aspc_jet_pack (cast `/Game/_GameManager/PC_JetPack` (`GameplayStatics.GetPlayerController` 0))
    (:`then`
      (set `self.PC Ref` _aspc_jet_pack))
    (:`CastFailed`
      _))
  (bind _asbp_third_person_character (cast `/Game/ThirdPerson/Blueprints/BP_ThirdPersonCharacter` (`GameplayStatics.GetPlayerCharacter` 0))
    (:`then`
      (set `self.Player Ref` _asbp_third_person_character))
    (:`CastFailed`
      _))
  (bind _asgm_jetpack (cast `/Game/_GameManager/GM_Jetpack` (`GameplayStatics.GetGameMode`)))
  (set `self.As GM Jetpack` _asgm_jetpack))

(event `self.ReceiveTick`
  (params (DeltaSeconds :type "Float (single-precision)"))
  (bind _returnvalue (`self.K2_GetActorLocation` (`GameplayStatics.GetPlayerPawn` 0)))
  ;[1 1 1] Move
  (`|ExecutionSequence`
    (:`then_0`
      (if (`self.Enabled`)
        (if (not (`self.StopMovement`))
          (`KismetSystemLibrary.MoveComponentTo` (`self.CapsuleComponent`) _returnvalue (struct) false false (/ (`KismetMathLibrary.VSize` (- (`self.K2_GetActorLocation`) _returnvalue)) (`self.Enemy Speed`))))))
    (:`then_1`
      (bind _player_ref (`self.Player Ref`)
        (:`then`
          (if (`/Game/ThirdPerson/Blueprints/BP_ThirdPersonCharacter.HasShip?` _player_ref)
            (bind _head_kill_box (`self.Head Kill Box`)
              (:`then`
                (`ActorComponent.SetActive` _head_kill_box false true))
              (:`else`))
            (else
              (bind _head_kill_box_2 (`self.Head Kill Box`)
                (:`then`
                  (`ActorComponent.SetActive` _head_kill_box_2 true true))
                (:`else`)))))
        (:`else`)))))

(event `self.Head Kill Box.OnComponentBeginOverlap`
  (params (OverlappedComponent :type "PrimitiveComponent Object Reference") (OtherActor :type "Actor Object Reference") (OtherComp :type "PrimitiveComponent Object Reference") (OtherBodyIndex :type Integer) (bFromSweep :type Boolean) (SweepResult :type "HitResult Structure (by ref)"))
  ;[1 1 1] Kill With Player
  (bind _asbp_third_person_character (cast `/Game/ThirdPerson/Blueprints/BP_ThirdPersonCharacter` OtherActor))
  (if (`self.ActorHasTag` _asbp_third_person_character "Player")
    (`/Game/_GameManager/GM_Jetpack.GainScore` (`self.As GM Jetpack`) (`self.Score Kill Enemy`))
    (`self.Destroy Box Score`)
    (`self.Show Score Kill`)
    (bind (_velocity_x _velocity_y _velocity_z) (`KismetMathLibrary.BreakVector` (`MovementComponent.Velocity` (`Character.CharacterMovement` _asbp_third_person_character))))
    (`self.LaunchCharacter` (`self.Player Ref`) (`KismetMathLibrary.MakeVector` 0.0 0.0 (+ (`self.Bounce Force`) (`KismetMathLibrary.Abs` _velocity_z))) false false)
    (bind _screentrigger (`self.ScreenTrigger` :!label _label)
      (:`then`
        (`/Game/MapElements/BP_ScreenTrigger.UpdateScreen` _screentrigger self))
      (:`else`
        _))
    (`self.DieFeedbacks`)))

(event `self.KillBox.OnComponentBeginOverlap`
  (params (OverlappedComponent :type "PrimitiveComponent Object Reference") (OtherActor :type "Actor Object Reference") (OtherComp :type "PrimitiveComponent Object Reference") (OtherBodyIndex :type Integer) (bFromSweep :type Boolean) (SweepResult :type "HitResult Structure (by ref)"))
  ;[1 1 1] Kill With Ship
  (bind _asbp_spaceship (cast `/Game/Spaceship/BP_Spaceship` OtherActor)
    (:`then`
      (if (`self.ActorHasTag` _asbp_spaceship "Player")
        (if (not (`/Game/Spaceship/BP_Spaceship.Invincible?` _asbp_spaceship))
          (`self.Player Repulse Hit Enemy` :!label _label_2)
          (`/Game/_GameManager/PC_JetPack.Decrement Health` (`self.PC Ref`)))))
    (:`CastFailed`
      (cast `/Game/Spaceship/BP_Projectile` OtherActor
        (:`then`
          (`self.Destroy Box Score`)
          (`/Game/_GameManager/GM_Jetpack.GainScore` (`self.As GM Jetpack`) (`self.Score Kill Enemy`))
          (goto _label))
        (:`CastFailed`
          (cast `/Game/ThirdPerson/Blueprints/BP_ThirdPersonCharacter` OtherActor)
          (goto _label_2))))))

(event `DieFeedbacks`
  (bind _returnvalue (`self.K2_GetActorLocation`))
  ;[1 1 1] DieFeedbacks
  (`GameplayStatics.PlaySound2D` "/Game/SoundEffect/Enemy/Enemy_Death_Sound_Effect.Enemy_Death_Sound_Effect" 1.0 1.0 0.0 null null)
  (`|ExecutionSequence`
    (:`then_0`
      (bind (_direction _alpha) (`Timeline|Dieexplosion` :!via `PlayFromStart`)
        (:`Update`
          (`self.SetActorScale3D` (`KismetMathLibrary.VLerp` (`self.GetActorScale3D`) (2.0 2.0 2.0) _alpha)))
        (:`Finished`
          ;[1 1 1] When Die Anim finished
          (`NiagaraFunctionLibrary.SpawnSystemAtLocation` "/Game/Feedbacks/NS_EnemyDie.NS_EnemyDie" _returnvalue)
          (`/Game/SystemAndBlueprints/3DWidgetHitEffect/AC_TakeDamageHitFx.SpawnWidget` (`self.AC_TakeDamageHitFx`) (`self.Score Kill Enemy`) _returnvalue)
          (`KismetSystemLibrary.PrintString` "Widget Spawned")
          ;[1 1 1] Destroy The enemy
          (`self.K2_DestroyActor`))))
    (:`then_1`
      ;[1 1 1] Dissolve Effect
      (bind (_direction_2 _newtrack_0) (`Timeline|Timeline` :!via `PlayFromStart`)
        (:`Update`
          (`MeshComponent.SetScalarParameterValueOnMaterials` (`self.Cube`) "Progress" _newtrack_0))))))

(fn `UserConstructionScript`)