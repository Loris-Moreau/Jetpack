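; Chasing enemy for the jetpack game that moves toward the player pawn at a set speed while enabled.
; A head-box stomp awards score and bounces the character, while body-box contact with character or player ship repulses it and costs health.
; Stomps and projectile hits remove both hitboxes, stop movement, show score text and play sounds.
; After a short delay, the killed enemy notifies its ScreenTrigger and destroys itself.
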(event `Player Repulse Hit Enemy`
  (bind _returnvalue (`GameplayStatics.GetPlayerPawn` 0))
  (bind (_returnvalue_x _returnvalue_y) (`KismetMathLibrary.BreakVector` (`SceneComponent.GetForwardVector` (`Actor.RootComponent` _returnvalue))))
  ;[1 1 1] Repusle Player
  (bind _player_ref (`self.Player Ref`)
    (:`then`
      (`self.LaunchCharacter` _player_ref (`KismetMathLibrary.MakeVector` 0.0 (* 50.0 _returnvalue_y)) true true))
    (:`else`
      (bind _asbp_spaceship (cast `/Game/Spaceship/BP_Spaceship` _returnvalue))
      (`PrimitiveComponent.AddImpulse` (`/Game/Spaceship/BP_Spaceship.Box` _asbp_spaceship) (0.0 -75.0 0.0) "None" false))))

(event `Stop Movement`
  ;[1 1 1] Stop Move
  (set `self.StopMovement` true)
  (if (`self.Enabled`)
    (`KismetSystemLibrary.MoveComponentTo` (`self.CapsuleComponent`) (`self.K2_GetActorLocation`))))

(event `Destroy Box Score`
  (`ActorComponent.K2_DestroyComponent` (`self.KillBox`))
  (`ActorComponent.K2_DestroyComponent` (`self.Head Kill Box`)))

(event `Show Score Dash Kill`
  (bind _scoretxt (`self.ScoreTXT`))
  (`TextRenderComponent.K2_SetText` _scoretxt (`|FormatText` "+ {score}" (`self.Score Kill Dash`)))
  (`SceneComponent.SetVisibility` _scoretxt true false)
  (`SceneComponent.SetVisibility` (`self.Cube`) false false)
  (`self.Stop Movement`))

(event `Show Score Kill`
  (bind _scoretxt (`self.ScoreTXT`))
  (`TextRenderComponent.K2_SetText` _scoretxt (`|FormatText` "+ {score}" (`self.Score Kill Enemy`)))
  (`SceneComponent.SetVisibility` _scoretxt true false)
  (`SceneComponent.SetVisibility` (`self.Cube`) false false)
  (`self.Stop Movement`))

(event `self.ReceiveBeginPlay`
  (`SceneComponent.SetVisibility` (`self.ScoreTXT`) false false)
  (bind _asbp_third_person_character (cast `/Game/ThirdPerson/Blueprints/BP_ThirdPersonCharacter` (`GameplayStatics.GetPlayerCharacter` 0))
    (:`then`
      (set `self.Player Ref` _asbp_third_person_character))
    (:`CastFailed`
      _))
  (bind _aspc_jet_pack (cast `/Game/_GameManager/PC_JetPack` (`GameplayStatics.GetPlayerController` 0))
    (:`then`
      (set `self.PC Ref` _aspc_jet_pack))
    (:`CastFailed`
      _))
  (bind _asgm_jetpack (cast `/Game/_GameManager/GM_Jetpack` (`GameplayStatics.GetGameMode`)))
  (set `self.As GM Jetpack` _asgm_jetpack))

(event `self.ReceiveTick`
  (params (DeltaSeconds :type "Float (single-precision)"))
  (bind _returnvalue (`self.K2_GetActorLocation` (`GameplayStatics.GetPlayerPawn` 0)))
  ;[1 1 1] Move
  (if (`self.Enabled`)
    (if (not (`self.StopMovement`))
      (`KismetSystemLibrary.MoveComponentTo` (`self.CapsuleComponent`) _returnvalue (struct) false false (/ (`KismetMathLibrary.VSize` (- (`self.K2_GetActorLocation`) _returnvalue)) (`self.Enemy Speed`))))))

(event `self.Head Kill Box.OnComponentBeginOverlap`
  (params (OverlappedComponent :type "PrimitiveComponent Object Reference") (OtherActor :type "Actor Object Reference") (OtherComp :type "PrimitiveComponent Object Reference") (OtherBodyIndex :type Integer) (bFromSweep :type Boolean) (SweepResult :type "HitResult Structure (by ref)"))
  (bind (_velocity_x _velocity_y _velocity_z) (`KismetMathLibrary.BreakVector` (`MovementComponent.Velocity` (`Character.CharacterMovement` (`self.Player Ref`)))))
  (bind _asbp_third_person_character (cast `/Game/ThirdPerson/Blueprints/BP_ThirdPersonCharacter` OtherActor))
  (if (`self.ActorHasTag` _asbp_third_person_character "Player")
    (`/Game/_GameManager/GM_Jetpack.GainScore` (`self.As GM Jetpack`) (`self.Score Kill Enemy`))
    (`self.Destroy Box Score`)
    (`self.Show Score Kill`)
    (`self.LaunchCharacter` (`self.Player Ref`) (`KismetMathLibrary.MakeVector` 0.0 0.0 (+ (`self.Bounce Force`) (`KismetMathLibrary.Abs` _velocity_z))) false false)
    ;[0 1 0.03793] Sound
    (`GameplayStatics.PlaySound2D` "/Game/SoundEffect/Enemy/Add_Score_Sound_Effect.Add_Score_Sound_Effect" 1.0 1.0 0.0 null null :!label _label)
    (`|ExecutionSequence`
      (:`then_0`
        (bind (_direction _newtrack_0) (`Timeline|Timeline` :!via `PlayFromStart`)
          (:`Update`
            (`MeshComponent.SetScalarParameterValueOnMaterials` (`self.Cube`) "Progress" _newtrack_0))))
      (:`then_1`
        (`KismetSystemLibrary.Delay` 0.2)
        (`GameplayStatics.PlaySound2D` "/Game/SoundEffect/Enemy/Enemy_Death_Sound_Effect.Enemy_Death_Sound_Effect" 1.0 1.0 0.0 null null)
        (`/Game/MapElements/BP_ScreenTrigger.UpdateScreen` (`self.ScreenTrigger`) self)
        (`self.K2_DestroyActor`)))))

(event `self.KillBox.OnComponentBeginOverlap`
  (params (OverlappedComponent :type "PrimitiveComponent Object Reference") (OtherActor :type "Actor Object Reference") (OtherComp :type "PrimitiveComponent Object Reference") (OtherBodyIndex :type Integer) (bFromSweep :type Boolean) (SweepResult :type "HitResult Structure (by ref)"))
  ;[1 1 1] Kill With Ship
  (bind _asbp_spaceship (cast `/Game/Spaceship/BP_Spaceship` OtherActor)
    (:`then`
      (if (`self.ActorHasTag` _asbp_spaceship "Player")
        (`self.Player Repulse Hit Enemy` :!label _label_2)
        (`/Game/_GameManager/PC_JetPack.Decrement Health` (`self.PC Ref`))))
    (:`CastFailed`
      (cast `/Game/Spaceship/BP_Projectile` OtherActor
        (:`then`
          (`self.Destroy Box Score`)
          (`self.Show Score Dash Kill`)
          (goto _label))
        (:`CastFailed`
          (cast `/Game/ThirdPerson/Blueprints/BP_ThirdPersonCharacter` OtherActor)
          (goto _label_2))))))

(event `self.KillBox.OnComponentEndOverlap`
  (params (OverlappedComponent :type "PrimitiveComponent Object Reference") (OtherActor :type "Actor Object Reference") (OtherComp :type "PrimitiveComponent Object Reference") (OtherBodyIndex :type Integer))
  (if (`self.ActorHasTag` OtherActor "Player")
    (`KismetSystemLibrary.Delay` 0.3)))

(fn `UserConstructionScript`)