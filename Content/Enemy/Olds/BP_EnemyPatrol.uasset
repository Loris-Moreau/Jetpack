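; Patrolling enemy that moves along a referenced spline via a timeline and awards score when the player kills it.
; Overlapping the head box kills it and bounces the player upward; the body box kills it only during a dash, otherwise costing player health.
; A kill removes both boxes, stops movement, shows the score text, hides the cube while running a dissolve, plays sounds and updates an optional screen trigger.
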(event `self.ReceiveTick`
  (params (DeltaSeconds :type "Float (single-precision)")))

(event `Player Repulse Hit Enemy`
  ;[1 1 1] Repusle Player
)

(event `Destroy Box Score`
  (`ActorComponent.K2_DestroyComponent` (`self.Kill Head Box`))
  (`ActorComponent.K2_DestroyComponent` (`self.KillBox`)))

(event `Show Score Dash Kill`
  (bind _scoretxt (`self.ScoreTXT`))
  (`TextRenderComponent.K2_SetText` _scoretxt (`|FormatText` "+ {score}" (`self.Score Kill Dash`)))
  (`SceneComponent.SetVisibility` _scoretxt true false)
  (`SceneComponent.SetVisibility` (`self.Cube`) false false)
  (`TimelineComponent.Stop` (`self.MoveObjectT`)))

(event `Show Score Kill`
  (bind _scoretxt (`self.ScoreTXT`))
  (`TextRenderComponent.K2_SetText` _scoretxt (`|FormatText` "+ {score}" (`self.Score Kill Enemy`)))
  (`SceneComponent.SetVisibility` _scoretxt true false)
  (`SceneComponent.SetVisibility` (`self.Cube`) false false)
  (`TimelineComponent.Stop` (`self.MoveObjectT`)))

(event `self.ReceiveBeginPlay`
  ;[1 1 1] Define Spline REF
  (set `self.SplineREF` (`self.SplineREF`))
  (`SceneComponent.SetVisibility` (`self.ScoreTXT`) false false)
  (bind _asbp_third_person_character (cast `/Game/ThirdPerson/Blueprints/BP_ThirdPersonCharacter` (`GameplayStatics.GetPlayerCharacter` 0))
    (:`then`
      (set `self.Player Ref` _asbp_third_person_character))
    (:`CastFailed`
      _))
  (bind _aspc_jet_pack (cast `/Game/_GameManager/PC_JetPack` (`GameplayStatics.GetPlayerController` 0))
    (:`then`
      (set `self.PC Ref` _aspc_jet_pack))
    (:`CastFailed`
      _))
  (bind _asgm_jetpack (cast `/Game/_GameManager/GM_Jetpack` (`GameplayStatics.GetGameMode`)))
  (set `self.As GM Jetpack` _asgm_jetpack))

(event `Move Object`
  ;[1 1 1] Move Enemy on Spline
  (`TimelineComponent.SetPlayRate` (`self.MoveObjectT`) (/ 1.0 (`self.Time To Complete`)))
  (bind (_direction _movetrack) (`Timeline|MoveObjectT` :!via `PlayFromStart`)
    (:`Update`
      (`self.K2_SetActorTransform` (`KismetMathLibrary.MakeTransform` (`SplineComponent.GetLocationAtDistanceAlongSpline` (`/Game/Enemy/BP_Spline.Spline` (`self.SplineREF`)) (`KismetMathLibrary.Lerp` 0.0 (`SplineComponent.GetSplineLength` (`/Game/Enemy/BP_Spline.Spline` (`self.SplineREF`))) _movetrack) "World")) true))))

(event `self.Kill Head Box.OnComponentBeginOverlap`
  (params (OverlappedComponent :type "PrimitiveComponent Object Reference") (OtherActor :type "Actor Object Reference") (OtherComp :type "PrimitiveComponent Object Reference") (OtherBodyIndex :type Integer) (bFromSweep :type Boolean) (SweepResult :type "HitResult Structure (by ref)"))
  (bind _cube (`self.Cube`))
  (bind _returnvalue_name (break `MaterialParameterInfo` (`MaterialInterface.GetParameterInfo` (`PrimitiveComponent.GetMaterial` _cube 0) "GlobalParameter" "Progress" null)))
  (bind (_velocity_x _velocity_y _velocity_z) (`KismetMathLibrary.BreakVector` (`MovementComponent.Velocity` (`Character.CharacterMovement` (`self.Player Ref`)))))
  (cast `/Game/ThirdPerson/Blueprints/BP_ThirdPersonCharacter` OtherActor)
  (if (`self.ActorHasTag` OtherActor "Player")
    ;[1 1 1] Add Scoring Sys
    (`/Game/_GameManager/GM_Jetpack.GainScore` (`self.As GM Jetpack`) (`self.Score Kill Enemy`))
    (`self.Destroy Box Score`)
    (`self.Show Score Kill`)
    (`Character.LaunchCharacter` (`self.Player Ref`) (`KismetMathLibrary.MakeVector` 0.0 0.0 (+ (`self.Bounce Force`) (`KismetMathLibrary.Abs` _velocity_z))) false false)
    (`GameplayStatics.PlaySound2D` "/Game/SoundEffect/Enemy/Add_Score_Sound_Effect.Add_Score_Sound_Effect" 1.0 1.0 0.0 null null :!label _label)
    (`|ExecutionSequence`
      (:`then_0`
        (bind (_direction _newtrack_0) (`Timeline|Dissolve` :!via `PlayFromStart`)
          (:`Update`
            (`MeshComponent.SetScalarParameterValueOnMaterials` _cube _returnvalue_name _newtrack_0))))
      (:`then_1`
        (`KismetSystemLibrary.Delay` 0.25)
        (`GameplayStatics.PlaySound2D` "/Game/SoundEffect/Enemy/Enemy_Death_Sound_Effect.Enemy_Death_Sound_Effect" 1.0 1.0 0.0 null null)
        (bind _screentrigger (`self.ScreenTrigger`)
          (:`then`
            (`/Game/MapElements/BP_ScreenTrigger.UpdateScreen` _screentrigger self))
          (:`else`))))))

(event `self.KillBox.OnComponentBeginOverlap`
  (params (OverlappedComponent :type "PrimitiveComponent Object Reference") (OtherActor :type "Actor Object Reference") (OtherComp :type "PrimitiveComponent Object Reference") (OtherBodyIndex :type Integer) (bFromSweep :type Boolean) (SweepResult :type "HitResult Structure (by ref)"))
  (bind _pc_ref (`self.PC Ref`))
  ;[1 1 1] Kill With Dash
  (if (`self.ActorHasTag` OtherActor "Player")
    (if (`/Game/_GameManager/PC_JetPack.Is Dashing` _pc_ref)
      (`/Game/_GameManager/GM_Jetpack.GainScore` (`self.As GM Jetpack`) (`self.Score Kill Dash`))
      (`self.Destroy Box Score`)
      (`self.Show Score Dash Kill`)
      (goto _label)
      (else
        (`/Game/_GameManager/PC_JetPack.Decrement Health` _pc_ref)
        (`self.Player Repulse Hit Enemy`)))))

(event `self.KillBox.OnComponentEndOverlap`
  (params (OverlappedComponent :type "PrimitiveComponent Object Reference") (OtherActor :type "Actor Object Reference") (OtherComp :type "PrimitiveComponent Object Reference") (OtherBodyIndex :type Integer))
  (if (`self.ActorHasTag` OtherActor "Player")
    (`KismetSystemLibrary.Delay` 0.3)))

(event `self.ReceiveAnyDamage`
  (params (Damage :type "Float (single-precision)") (DamageType :type "DamageType Object Reference") (InstigatedBy :type "Controller Object Reference") (DamageCauser :type "Actor Object Reference")))

(fn `UserConstructionScript`)