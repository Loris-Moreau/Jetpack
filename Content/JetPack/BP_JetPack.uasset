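; Jetpack pickup that bobs in the level until the player overlaps it, then attaches to their pelvis socket.
; BeginPlay copies its dash, gravity-increase and thrust tuning onto BP_ThirdPersonCharacter, before any pickup occurs.
; Tick drives the bob with a Delay-fed FlipFlop until pickup, then stops the rotating movement.
; While the character reports the jetpack active, Tick activates both Niagara effects and plays controller force feedback.
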(event `self.ReceiveBeginPlay`
  (bind _player_ref (`self.Player Ref`))
  (bind _asbp_third_person_character (cast `/Game/ThirdPerson/Blueprints/BP_ThirdPersonCharacter` (`GameplayStatics.GetPlayerPawn` 0)))
  (set `self.Player Ref` _asbp_third_person_character)
  (`ActorComponent.Deactivate` (`self.Niagara`))
  (`ActorComponent.Deactivate` (`self.Niagara1`))
  (set `/Game/ThirdPerson/Blueprints/BP_ThirdPersonCharacter.Dash Strength` (`self.Dash Strength`) _player_ref)
  (set `/Game/ThirdPerson/Blueprints/BP_ThirdPersonCharacter.Dash Cooldown Time` (`self.Dash Cooldown`) _player_ref)
  (set `/Game/ThirdPerson/Blueprints/BP_ThirdPersonCharacter.Grav Increase Factor` (`self.Grav Increase Factor`) _player_ref)
  (set `/Game/ThirdPerson/Blueprints/BP_ThirdPersonCharacter.Grav Increase Max` (`self.Grav Increase Max`) _player_ref)
  (set `/Game/ThirdPerson/Blueprints/BP_ThirdPersonCharacter.Grav Increase Speed` (`self.Grav Increase Speed`) _player_ref)
  (set `/Game/ThirdPerson/Blueprints/BP_ThirdPersonCharacter.Jetpack Up Velocity` (`self.Jetpack up Velocity`) _player_ref))

(event `self.ReceiveTick`
  (params (DeltaSeconds :type "Float (single-precision)"))
  ;[0.25 0.25 0.25] Pickup Logic
  (if (`/Game/ThirdPerson/Blueprints/BP_ThirdPersonCharacter.Jetpacked Picked up` (`self.Player Ref`))
    (`ActorComponent.Deactivate` (`self.RotatingMovement`))
    ;[3 0.7453 0.267] FX
    (if (`/Game/ThirdPerson/Blueprints/BP_ThirdPersonCharacter.Is Jetpacked Active` (`self.Player Ref`))
      (`ActorComponent.Activate` (`self.Niagara`) true)
      (`ActorComponent.Activate` (`self.Niagara1`) true)
      (`PlayerController.PlayDynamicForceFeedback` (`GameplayStatics.GetPlayerController` 0) 0.5 0.45 true true true true))
    (else
      (`|ExecutionSequence`
        (:`then_0`
          (`KismetSystemLibrary.Delay` (`self.Pickup Swing Delay`))
          (bind _isa (`/Engine/EditorBlueprintResources/StandardMacros.FlipFlop`)
            (:`A`
              _)
            (:`B`
              _))
          (set `self.Dir` _isa))
        (:`then_1`
          (if (`self.Dir`)
            (`self.K2_AddActorLocalOffset` (`KismetMathLibrary.MakeVector` 0.0 0.0 (`self.Pickup Offset`)))
            (else
              (`self.K2_AddActorLocalOffset` (`KismetMathLibrary.MakeVector` 0.0 0.0 (* (`self.Pickup Offset`) -1.0))))))))))

(event `self.Box.OnComponentBeginOverlap`
  (params (OverlappedComponent :type "PrimitiveComponent Object Reference") (OtherActor :type "Actor Object Reference") (OtherComp :type "PrimitiveComponent Object Reference") (OtherBodyIndex :type Integer) (bFromSweep :type Boolean) (SweepResult :type "HitResult Structure (by ref)"))
  ;[0.25 0.25 0.25] Pickup Logic
  (bind _player_ref (`self.Player Ref`)
    (:`then`
      (if (== _player_ref OtherActor)
        (set `/Game/ThirdPerson/Blueprints/BP_ThirdPersonCharacter.Jetpacked Picked up` true (`self.Player Ref`))
        (`ActorComponent.SetActive` (`self.Box`) false false)
        (`self.K2_AttachToActor` (`self.Player Ref`) "pelvis" "SnapToTarget" "SnapToTarget" "SnapToTarget")
        (`self.K2_AddActorLocalOffset` (-25.0 0.0 30.0))))
    (:`else`)))

(fn `UserConstructionScript`)