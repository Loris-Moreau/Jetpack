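; BP_Camera is a camera actor for the Jetpack game that makes a one-time vertical move to a requested height.
; MoveCam is guarded by HasMoved, reads the starting Z from the GM_Jetpack game mode's GameCam, and scales the timeline's play rate by BlendTime.
; Each timeline update sets this actor's location, lerping Z toward the target while taking X and Y from GameCam.
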(event `MoveCam`
  (params (Height :type "Float (double-precision)"))
  (bind (_returnvalue_x _returnvalue_y _returnvalue_z) (`KismetMathLibrary.BreakVector` (`self.K2_GetActorLocation` (`/Game/_GameManager/GM_Jetpack.GameCam` (cast `/Game/_GameManager/GM_Jetpack` (`GameplayStatics.GetGameMode`) :!pure true)))))
  (bind (_returnvalue_x_2 _returnvalue_y_2) (`KismetMathLibrary.BreakVector` (`self.K2_GetActorLocation` (`/Game/_GameManager/GM_Jetpack.GameCam` (cast `/Game/_GameManager/GM_Jetpack` (`GameplayStatics.GetGameMode`) :!pure true)))))
  (if (not (`self.HasMoved?`))
    (set `self.HasMoved?` true)
    (set `self.CurrHeight` _returnvalue_z)
    (`TimelineComponent.SetPlayRate` (`self.MoveCam_T`) (/ 1.0 (`self.BlendTime`)))
    (bind (_direction _movecamtrack) (`Timeline|MoveCam_T` :!via `PlayFromStart`)
      (:`Update`
        (`self.K2_SetActorLocation` (`KismetMathLibrary.MakeVector` _returnvalue_x_2 _returnvalue_y_2 (`KismetMathLibrary.Lerp` (`self.CurrHeight`) Height _movecamtrack)))))))

(fn `UserConstructionScript`)