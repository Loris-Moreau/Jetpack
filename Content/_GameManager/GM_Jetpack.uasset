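; GM_Jetpack is a game manager Blueprint, apparently for a jetpack game, that sets up the gameplay camera.
; On BeginPlay it spawns a BP_Camera at CameraSpawnPosition, stores it as GameCam, activates its camera component and makes it player 0's view target.
; Tick is empty, and an unconnected debug print of the camera's moved state and height never runs.
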(event `self.ReceiveBeginPlay`
  (bind _returnvalue (`|SpawnActorFromClass` "/Game/_GameManager/BP_Camera.BP_Camera_C" (`KismetMathLibrary.MakeTransform` (`self.CameraSpawnPosition`)) "Undefined" "MultiplyWithRoot" null null))
  (bind _output_get (set `self.GameCam` _returnvalue))
  (`ActorComponent.SetActive` (`/Game/_GameManager/BP_Camera.Camera` _returnvalue) true true)
  (`PlayerController.SetViewTargetWithBlend` (`GameplayStatics.GetPlayerController` 0) _output_get 0.0 "VTBlend_Linear" 0.0 false))

(event `self.ReceiveTick`
  (params (DeltaSeconds :type "Float (single-precision)")))

(fn `UserConstructionScript`)