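; BP_Port is a port actor that switches player control from the spaceship back to the third-person character.
; On BeginPlay it caches the JetPack player controller and the third-person character.
; The first BP_Spaceship overlap moves that character to the current pawn's Y and raised Z, keeping its own X, rotation and scale, then possesses it.
; A DoOnce with no reset limits the handover to a single time.
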(event `self.ReceiveBeginPlay`
  (bind _aspc_jet_pack (cast `/Game/_GameManager/PC_JetPack` (`GameplayStatics.GetPlayerController` 0)))
  (set `self.PC Ref` _aspc_jet_pack)
  (bind _asbp_third_person_character (cast `/Game/ThirdPerson/Blueprints/BP_ThirdPersonCharacter` (`GameplayStatics.GetPlayerCharacter` 0)))
  (set `self.TPS Chara Ref` _asbp_third_person_character))

(event `self.ReceiveActorBeginOverlap`
  (params (OtherActor :type "Actor Object Reference"))
  (bind _returnvalue (`GameplayStatics.GetPlayerController` 0))
  (bind _returnvalue_2 (`self.GetTransform` (`self.TPS Chara Ref`)))
  (bind _returnvalue_3 (`self.GetTransform` (`GameplayStatics.GetPlayerPawn` 0)))
  (cast `/Game/Spaceship/BP_Spaceship` OtherActor)
  (`/Engine/EditorBlueprintResources/StandardMacros.DoOnce` false
    (:`Completed`
      (`self.K2_SetActorTransform` (`self.TPS Chara Ref`) (`KismetMathLibrary.MakeTransform` (`KismetMathLibrary.MakeVector` (.x (.location _returnvalue_2)) (.y (.location _returnvalue_3)) (+ (.z (.location _returnvalue_3)) 100.0)) (.rotation _returnvalue_2) (.scale _returnvalue_2)) false false)
      (`Controller.UnPossess` _returnvalue)
      (`Controller.Possess` _returnvalue (`self.TPS Chara Ref`)))))

(fn `UserConstructionScript`)