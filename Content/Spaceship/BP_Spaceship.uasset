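; BP_Spaceship is a spaceship that the player can possess in place of the third-person character.
; On BeginPlay it caches the player's BP_ThirdPersonCharacter, and on possession it stores the new player controller.
; Possession flags the character as having a ship, zeroes its gravity and hides its mesh and jetpack.
; Unpossession clears the flag, restores base gravity and shows both again.
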(event `self.ReceiveBeginPlay`
  (bind _asbp_third_person_character (cast `/Game/ThirdPerson/Blueprints/BP_ThirdPersonCharacter` (`GameplayStatics.GetPlayerCharacter` 0)))
  (set `self.TPChara Ref` _asbp_third_person_character))

(event `self.ReceivePossessed`
  (params (NewController :type "Controller Object Reference"))
  (bind _tpchara_ref (`self.TPChara Ref`))
  (bind _tpchara_ref_2 (`self.TPChara Ref`))
  (bind _asplayer_controller (cast `PlayerController` NewController))
  (set `self.Player Controller Ref` _asplayer_controller)
  (set `/Game/ThirdPerson/Blueprints/BP_ThirdPersonCharacter.HasShip?` true _tpchara_ref)
  (set `CharacterMovementComponent.GravityScale` 0.0 (`Character.CharacterMovement` _tpchara_ref))
  (`SceneComponent.SetVisibility` (`Character.Mesh` _tpchara_ref_2) false true)
  (`SceneComponent.SetVisibility` (`/Game/JetPack/BP_JetPack.Cube` (`/Game/ThirdPerson/Blueprints/BP_ThirdPersonCharacter.Jetpack Ref` _tpchara_ref_2)) false true))

(event `self.ReceiveUnpossessed`
  (params (OldController :type "Controller Object Reference"))
  (bind _tpchara_ref (`self.TPChara Ref`))
  (bind _tpchara_ref_2 (`self.TPChara Ref`))
  (set `/Game/ThirdPerson/Blueprints/BP_ThirdPersonCharacter.HasShip?` false _tpchara_ref)
  (set `CharacterMovementComponent.GravityScale` (`/Game/ThirdPerson/Blueprints/BP_ThirdPersonCharacter.Base Gravity` _tpchara_ref) (`Character.CharacterMovement` _tpchara_ref))
  (`SceneComponent.SetVisibility` (`Character.Mesh` _tpchara_ref_2) true true)
  (`SceneComponent.SetVisibility` (`/Game/JetPack/BP_JetPack.Cube` (`/Game/ThirdPerson/Blueprints/BP_ThirdPersonCharacter.Jetpack Ref` _tpchara_ref_2)) true true))

(fn `UserConstructionScript`)