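; Gun component for the spaceship that fires projectiles from a billboard marker on the fire input.
; Each shot spawns a BP_Projectile with a fixed rotation, triggers the spaceship's shoot animation and plays sound and Niagara effects at the muzzle.
; A Cooldown flag with a delay of one over FireRate limits the rate of fire.
; The move input does nothing; its direction-sign and offset logic is left disconnected.
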(event `EnhancedInput|/Game/ThirdPerson/Input/Actions/IA_Move`
  (params (ActionValue :type "Vector2D Structure") (ElapsedSeconds :type "Float (double-precision)") (TriggeredSeconds :type "Float (double-precision)") (InputAction :type "InputAction Object Reference" :default "/Game/ThirdPerson/Input/Actions/IA_Move.IA_Move")))

(event `EnhancedInput|/Game/ThirdPerson/Input/Actions/IA_Fire`
  (params (ActionValue :type Boolean) (ElapsedSeconds :type "Float (double-precision)") (TriggeredSeconds :type "Float (double-precision)") (InputAction :type "InputAction Object Reference" :default "/Game/ThirdPerson/Input/Actions/IA_Fire.IA_Fire"))
  (bind _returnvalue (`SceneComponent.K2_GetComponentLocation` (`self.GunPositionBillboard`)))
  (:`Triggered`
    (if (not (`self.Cooldown`))
      (`|SpawnActorFromClass` "/Game/Spaceship/BP_Projectile.BP_Projectile_C" (`KismetMathLibrary.MakeTransform` _returnvalue (`KismetMathLibrary.MakeRotator` 90.0)) "AlwaysSpawn" "MultiplyWithRoot" null (`GameplayStatics.GetPlayerPawn` 0))
      (bind _returnvalue_2 (`GameplayStatics.GetActorOfClass` "/Game/Spaceship/BP_Spaceship.BP_Spaceship_C"))
      (`/Game/Spaceship/BP_Spaceship.ShootAnim` _returnvalue_2)
      (`GameplayStatics.PlaySoundAtLocation` (`self.SFXShoot `) _returnvalue (struct) 1.0 1.0 0.0 null null null null)
      (`NiagaraFunctionLibrary.SpawnSystemAtLocation` (`self.VFXShoot `) _returnvalue)
      (set `self.Cooldown` true)
      (`KismetSystemLibrary.Delay` (/ 1.0 (`self.FireRate`)))
      (set `self.Cooldown` false))))