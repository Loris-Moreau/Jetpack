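; BP_Side is a screen-edge trigger that wraps the player to the other side of the screen.
; When BP_ThirdPersonCharacter overlaps its Box, it moves to the OtherSide actor's Y, offset by TPOffset in a direction set by Left, keeping its X and Z.
; Matching logic for BP_EnemySpot and BP_EnemyPatrol exists but is disconnected, so only the player character wraps.
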(event `self.Box.OnComponentBeginOverlap`
  (params (OverlappedComponent :type "PrimitiveComponent Object Reference") (OtherActor :type "Actor Object Reference") (OtherComp :type "PrimitiveComponent Object Reference") (OtherBodyIndex :type Integer) (bFromSweep :type Boolean) (SweepResult :type "HitResult Structure (by ref)"))
  (bind _tp_offset (`self.TP Offset`))
  (bind (_returnvalue_x _returnvalue_y) (`KismetMathLibrary.BreakVector` (`self.K2_GetActorLocation` (`self.OtherSide`))))
  ;[1 1 1] TP to other side of screen
  (bind _asbp_third_person_character (cast `/Game/ThirdPerson/Blueprints/BP_ThirdPersonCharacter` OtherActor))
  (if (`self.Left`)
    (bind (_returnvalue_x_2 _returnvalue_y_2 _returnvalue_z) (`KismetMathLibrary.BreakVector` (`self.K2_GetActorLocation` _asbp_third_person_character)))
    (`self.K2_SetActorLocation` _asbp_third_person_character (`KismetMathLibrary.MakeVector` _returnvalue_x_2 (- _returnvalue_y _tp_offset) _returnvalue_z) false false)
    (else
      (`self.K2_SetActorLocation` _asbp_third_person_character (`KismetMathLibrary.MakeVector` _returnvalue_x_2 (+ _returnvalue_y _tp_offset) _returnvalue_z) false false))))

(fn `UserConstructionScript`)