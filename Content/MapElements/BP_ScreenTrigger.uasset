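; BP_ScreenTrigger runs one enemy screen in the jetpack game, activating it when the player enters its box and completing it once every enemy is gone.
; On BeginPlay it links itself to both kill zones and four enemy sets (patrol, spot and their Spec variants), hiding enemies until triggered.
; Triggering enables kill-zone collision and starts the enemies.
; UpdateScreen removes and destroys enemies, then opens the top kill zone when all sets empty.
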(event `self.ReceiveBeginPlay`
  (`KismetSystemLibrary.Delay` 0.2)
  (set `/Game/MapElements/BP_KillZone.Screen` self (`self.KillZoneTop`))
  (set `/Game/MapElements/BP_KillZone.Screen` self (`self.KillZoneBottom`))
  (bind _result (`BlueprintSetLibrary.Set_ToArray` (`self.EnemyListSpline`)))
  (for _array_element _result
    (set `/Game/Enemy/BP_EnemyPatrol.ScreenTrigger` self _array_element)
    (`SceneComponent.SetHiddenInGame` (`/Game/Enemy/BP_EnemyPatrol.Cube` _array_element) true true))
  (bind _result_2 (`BlueprintSetLibrary.Set_ToArray` (`self.EnemyListSpot`)))
  (for _array_element_2 _result_2
    (set `/Game/Enemy/BP_EnemySpot.ScreenTrigger` self _array_element_2)
    (`SceneComponent.SetHiddenInGame` (`/Game/Enemy/BP_EnemySpot.Cube` _array_element_2) true true)
    (set `/Game/Enemy/BP_EnemySpot.Enabled` false _array_element_2))
  (bind _result_3 (`BlueprintSetLibrary.Set_ToArray` (`self.ListSpotSpec`)))
  (for _array_element_3 _result_3
    (set `/Game/Enemy/BP_EnemySpot_Spec.ScreenTrigger` self _array_element_3)
    (`SceneComponent.SetHiddenInGame` (`/Game/Enemy/BP_EnemySpot_Spec.Cube` _array_element_3) true true)
    (set `/Game/Enemy/BP_EnemySpot_Spec.Enabled` false _array_element_3))
  (bind _result_4 (`BlueprintSetLibrary.Set_ToArray` (`self.ListSplineSpec`)))
  (for _array_element_4 _result_4
    (set `/Game/Enemy/BP_EnemyPatrol_Spec.ScreenTrigger` self _array_element_4)
    (`SceneComponent.SetHiddenInGame` (`/Game/Enemy/BP_EnemyPatrol_Spec.Cube` _array_element_4) true true)))

(event `self.Box.OnComponentBeginOverlap`
  (params (OverlappedComponent :type "PrimitiveComponent Object Reference") (OtherActor :type "Actor Object Reference") (OtherComp :type "PrimitiveComponent Object Reference") (OtherBodyIndex :type Integer) (bFromSweep :type Boolean) (SweepResult :type "HitResult Structure (by ref)"))
  (cast `/Game/ThirdPerson/Blueprints/BP_ThirdPersonCharacter` OtherActor)
  (if (not (`self.Enabled?`))
    (set `self.Enabled?` true)
    (set `/Game/_GameManager/BP_Camera.HasMoved?` false (`/Game/_GameManager/GM_Jetpack.GameCam` (cast `/Game/_GameManager/GM_Jetpack` (`GameplayStatics.GetGameMode`) :!pure true)))
    (`PrimitiveComponent.SetCollisionEnabled` (`/Game/MapElements/BP_KillZone.Box` (`self.KillZoneBottom`)) "QueryAndPhysics")
    (`PrimitiveComponent.SetCollisionEnabled` (`/Game/MapElements/BP_KillZone.Cube` (`self.KillZoneTop`)) "QueryAndPhysics")
    (bind _result (`BlueprintSetLibrary.Set_ToArray` (`self.EnemyListSpline`)))
    (for _array_element _result
      (`SceneComponent.SetHiddenInGame` (`/Game/Enemy/BP_EnemyPatrol.Cube` _array_element) false true)
      (`/Game/Enemy/BP_EnemyPatrol.Move Object` _array_element))
    (bind _result_2 (`BlueprintSetLibrary.Set_ToArray` (`self.EnemyListSpot`)))
    (for _array_element_2 _result_2
      (set `/Game/Enemy/BP_EnemySpot.Enabled` true _array_element_2)
      (`SceneComponent.SetHiddenInGame` (`/Game/Enemy/BP_EnemySpot.Cube` _array_element_2) false true))
    (bind _result_3 (`BlueprintSetLibrary.Set_ToArray` (`self.ListSplineSpec`)))
    (for _array_element_3 _result_3
      (`SceneComponent.SetHiddenInGame` (`/Game/Enemy/BP_EnemyPatrol_Spec.Cube` _array_element_3) false true)
      (`/Game/Enemy/BP_EnemyPatrol_Spec.Move Object` _array_element_3))
    (bind _result_4 (`BlueprintSetLibrary.Set_ToArray` (`self.ListSpotSpec`)))
    (for _array_element_4 _result_4
      (set `/Game/Enemy/BP_EnemySpot_Spec.Enabled` true _array_element_4)
      (`SceneComponent.SetHiddenInGame` (`/Game/Enemy/BP_EnemySpot_Spec.Cube` _array_element_4) false true))
    ;[1 1 1] Spawn Sound
    (`GameplayStatics.PlaySound2D` null 1.0 1.0 0.0 null null)))

(event `UpdateScreen`
  (params (Actor :type "Actor Object Reference"))
  (`KismetSystemLibrary.Delay` (`self.CustomDelay`))
  (bind _asbp_enemy_patrol (cast `/Game/Enemy/BP_EnemyPatrol` Actor)
    (:`then`
      (`BlueprintSetLibrary.Set_Remove` (`self.EnemyListSpline`) _asbp_enemy_patrol)
      (`self.K2_DestroyActor` _asbp_enemy_patrol))
    (:`CastFailed`
      (bind _asbp_enemy_spot (cast `/Game/Enemy/BP_EnemySpot` Actor)
        (:`then`
          (`BlueprintSetLibrary.Set_Remove` (`self.EnemyListSpot`) _asbp_enemy_spot)
          (`self.K2_DestroyActor` _asbp_enemy_spot))
        (:`CastFailed`
          (bind _asbp_enemy_patrol_spec (cast `/Game/Enemy/BP_EnemyPatrol_Spec` Actor)
            (:`then`
              (`BlueprintSetLibrary.Set_Remove` (`self.ListSplineSpec`) _asbp_enemy_patrol_spec)
              (`self.K2_DestroyActor` _asbp_enemy_patrol_spec))
            (:`CastFailed`
              (bind _asbp_enemy_spot_spec (cast `/Game/Enemy/BP_EnemySpot_Spec` Actor))
              (`BlueprintSetLibrary.Set_Remove` (`self.ListSpotSpec`) _asbp_enemy_spot_spec)
              (`self.K2_DestroyActor` _asbp_enemy_spot_spec)))))))
  (if (and (`BlueprintSetLibrary.Set_IsEmpty` (`self.EnemyListSpline`)) (`BlueprintSetLibrary.Set_IsEmpty` (`self.EnemyListSpot`)) (`BlueprintSetLibrary.Set_IsEmpty` (`self.ListSpotSpec`)) (`BlueprintSetLibrary.Set_IsEmpty` (`self.ListSplineSpec`)))
    (`self.ScreenComplete`)))

(event `ScreenComplete`
  (bind _killzonetop (`self.KillZoneTop`))
  (`PrimitiveComponent.SetCollisionEnabled` (`/Game/MapElements/BP_KillZone.Box` _killzonetop) "NoCollision")
  (`PrimitiveComponent.SetCollisionEnabled` (`/Game/MapElements/BP_KillZone.Cube` _killzonetop) "NoCollision")
  ;[1 1 1] Next Screen Sound
  (`GameplayStatics.PlaySound2D` null 1.0 1.0 0.0 null null))

(fn `UserConstructionScript`)