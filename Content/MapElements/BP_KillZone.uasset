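; BP_KillZone is a kill-zone map element that is inert as wired: BeginPlay disables collision on its Cube and Box and caches the player character.
; The Box overlap event is empty, leaving the kill logic unreachable.
; That disconnected logic would award fall points and update Screen for four enemy types via chained casts.
; Separate orphaned nodes would decrement player health and teleport the player to Screen's respawn point.
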(event `self.ReceiveBeginPlay`
  ;[1 1 1] Disable on game start
  (`PrimitiveComponent.SetCollisionEnabled` (`self.Cube`) "NoCollision")
  (`PrimitiveComponent.SetCollisionEnabled` (`self.Box`) "NoCollision")
  (set `self.As BP Third Person Character` (cast `/Game/ThirdPerson/Blueprints/BP_ThirdPersonCharacter` (`Controller.K2_GetPawn` (`GameplayStatics.GetPlayerController` 0)) :!pure true)))

(event `self.Box.OnComponentBeginOverlap`
  (params (OverlappedComponent :type "PrimitiveComponent Object Reference") (OtherActor :type "Actor Object Reference") (OtherComp :type "PrimitiveComponent Object Reference") (OtherBodyIndex :type Integer) (bFromSweep :type Boolean) (SweepResult :type "HitResult Structure (by ref)")))

(fn `UserConstructionScript`)